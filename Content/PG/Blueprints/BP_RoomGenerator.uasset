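; Procedural level generator for a ball maze game, building a randomly sized square maze on BeginPlay and resetting the ball's position.
; Instanced meshes form floor and border walls, with a BP_FloorCollision actor per tile storing index and visited state as text.
; A randomized depth-first backtracking stack walks the tiles, adding an inner wall per step and culling outer-wall overlaps.
; Spawnable tiles then receive coin effects and set the game instance's key total.
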(event Custom|Generate%20Levels
  (bind _outactors (Actor|GetAllActorsOfClass "/Game/Blueprints/Pawn/BP_Ball.BP_Ball_C"))
  (Transformation|SetWorldLocation (Variables|/Game/Blueprints/Pawn/BP_Ball.BP_Ball_C|GetBallMesh (Utilities|Array|Get(acopy) _outactors)) "50.000000,50.000000,142.000000" false false)
  (Default|FixConstrain (Utilities|Array|Get(acopy) _outactors))
  (bind _output_get (Variables|Default|SetMXRow (Math|Random|RandomIntegerinRange 1 8)))
  (Variables|Default|SetMXCol _output_get)
  (CallFunction|MakeRoom)
  (CallFunction|PutWalls)
  (CallFunction|AddIndexes)
  (CallFunction|PushTCStack (Utilities|Array|Get(acopy) (Variables|Default|GetTile%20Collision%20Array)))
  (CallFunction|RandomMazeGeneration)
  (CallFunction|SetAllSpwanableTiles)
  (CallFunction|SpawnCoins))

(event EventBeginPlay
  (CallFunction|GenerateLevels))

(event Collision|EventActorBeginOverlap
  (params (OtherActor :type Actor%20Object%20Reference)))

(event EventDestroyed
  (for _array_element (Variables|Default|GetTile%20Collision%20Array)
    (Actor|DestroyActor _array_element)))

(fn ConstructionScript)

(fn MakeRoom
  (for _index (range 0 (- (Variables|Default|GetMXRow) 1))
    (for _index_2 (range 0 (- (Variables|Default|GetMXCol) 1))
      (Components|InstancedStaticMesh|AddInstance (Variables|Default|GetFloor) (Math|Transform|MakeTransform (Math|Vector|MakeVector (* _index (Variables|Default|GetTileLocation%20X)) (* _index_2 (Variables|Default|GetTileLocation%20Y)) 0.0) "0, 0, 0" "2.000000,2.000000,0.500000") true))))

(fn PutWalls
  (bind _wall (Variables|Default|GetWall))
  (bind _wall_2 (Variables|Default|GetWall))
  (Utilities|FlowControl|Sequence
    (:then_0
      ;[0 1 0.3618] Vertical Walls
      (for _index (range 0 (- (Variables|Default|GetMXRow) 1))
        (Components|InstancedStaticMesh|AddInstance _wall_2 (Math|Transform|MakeTransform (Math|Vector|MakeVector (+ (* _index (Variables|Default|GetTileLocation%20X)) 1e+02) 0.0 1e+02) "90.000000,-0.000000,90.000000" "2.000000,2.000000,0.125000") true)
        ;;[1 1 1] Parallel Wall X
        (Components|InstancedStaticMesh|AddInstance _wall_2 (Math|Transform|MakeTransform (Math|Vector|MakeVector (+ (* _index (Variables|Default|GetTileLocation%20X)) 1e+02) (* (Variables|Default|GetMXRow) 2e+02) 1e+02) "90.000000,-0.000000,90.000000" "2.000000,2.000000,0.125000") true)))
    (:then_1
      ;[1 0.6917 0] Column Walls
      (for _index_2 (range 0 (- (Variables|Default|GetMXCol) 1))
        (Components|InstancedStaticMesh|AddInstance _wall (Math|Transform|MakeTransform (Math|Vector|MakeVector 0.0 (+ (* _index_2 (Variables|Default|GetTileLocation%20Y)) 1e+02) 1e+02) "90.000000,-0.000000,0.000000" "2.000000,2.000000,0.125000") true)
        ;;[1 1 1] Parallel Wall
        (Components|InstancedStaticMesh|AddInstance _wall (Math|Transform|MakeTransform (Math|Vector|MakeVector (Math|Conversions|ToFloat(Integer) (* 200 (Variables|Default|GetMXCol))) (+ (* _index_2 (Variables|Default|GetTileLocation%20Y)) 1e+02) 1e+02) "90.000000,-0.000000,0.000000" "2.000000,2.000000,0.125000") true)))))

(fn AddIndexes
  (bind _asbp_maze_game_instance (Utilities|Casting|CastToBP_MazeGameInstance (Game|GetGameInstance)))
  (for _index (range 0 (- (Variables|Default|GetMXRow) 1))
    (for _index_2 (range 0 (- (Variables|Default|GetMXCol) 1))
      (bind _returnvalue (Game|SpawnActorfromClass "/Game/PG/Blueprints/BP_FloorCollision.BP_FloorCollision_C" (Math|Transform|MakeTransform (+ (Math|Vector|MakeVector (* _index (Variables|Default|GetTileLocation%20X)) (* _index_2 (Variables|Default|GetTileLocation%20Y)) 0.0) "100.000000,100.000000,0") "0, 0, 0" "1.000000,1.000000,1.010000") "Undefined" 0 0))
      (Rendering|Components|TextRender|SetText (Variables|/Game/PG/Blueprints/BP_FloorCollision.BP_FloorCollision_C|GetIndex%20Number _returnvalue) (Utilities|Text|ToText(String) (Utilities|String|ToString(Integer) (Variables|Default|GetTile%20Display%20Index))))
      (bind _returnvalue_2 (Utilities|Array|AddUnique (Variables|Default|GetTile%20Collision%20Array) _returnvalue))
      (Math|Integer|IncrementInt (Variables|Default|GetTile%20Display%20Index)
        (:%20%20
          (Development|PrintString (Utilities|String|Append "Index: " (Utilities|String|ToString(Integer) _returnvalue_2)) false))))))

(fn TestGetIndex
  (Development|PrintString (Utilities|String|ToString(Vector) (.location (.OutInstanceTransform (Components|InstancedStaticMesh|GetInstanceTransform (Variables|Default|GetFloor) 25 false)))) false true "(R=0.000000,G=0.660000,B=1.000000,A=1.000000)" 0.0))

(fn RandomMazeGeneration
  (if (Utilities|Array|IsEmpty (Variables|Default|GetTC_Stack)) :!label _label
    (return)
    (else
      (bind _output (CallFunction|FindVisitableTile (CallFunction|PeekTCStack) :!label _label_2))
      (Utilities|IsValid _output
        (:Is%20Valid
          (CallFunction|SpawnWalls _output)
          (CallFunction|PushTCStack _output)
          (goto _label_2))
        (:Is%20Not%20Valid
          (CallFunction|PopTCStack)
          (goto _label))))))

(fn FindVisitableTile
  (params (TargetTile :type BP%20Floor%20Collision%20Object%20Reference))
  (bind _output (CallFunction|GetBelowTile TargetTile))
  (bind _output_2 (CallFunction|GetAboveTile TargetTile))
  (bind _output_3 (CallFunction|GetRightTile TargetTile))
  (bind _output_4 (CallFunction|GetLeftTile TargetTile))
  (switch int (Math|Integer|%(Integer) (Math|Random|RandomIntegerinRange 0 200) 4) :!label _label
    (:0
      (if (CallFunction|IsVisitable _output)
        (return _output)
        (else
          (LocalVariables|SetHasVisited_1 true)
          (if (Math|Boolean|ANDBoolean (LocalVariables|GetHasVisited_4) (LocalVariables|GetHasVisited_1) (LocalVariables|GetHasVisited_2) (LocalVariables|GetHasVisited_3))
            (return 0)
            (else
              (goto _label))))))
    (:1
      (if (CallFunction|IsVisitable _output_2)
        (return _output_2)
        (else
          (LocalVariables|SetHasVisited_2 true)
          (if (Math|Boolean|ANDBoolean (LocalVariables|GetHasVisited_4) (LocalVariables|GetHasVisited_1) (LocalVariables|GetHasVisited_2) (LocalVariables|GetHasVisited_3))
            (return 0)
            (else
              (goto _label))))))
    (:2
      (if (CallFunction|IsVisitable _output_3)
        (return _output_3)
        (else
          (LocalVariables|SetHasVisited_3 true)
          (if (Math|Boolean|ANDBoolean (LocalVariables|GetHasVisited_4) (LocalVariables|GetHasVisited_1) (LocalVariables|GetHasVisited_2) (LocalVariables|GetHasVisited_3))
            (return 0)
            (else
              (goto _label))))))
    (:3
      (if (CallFunction|IsVisitable _output_4)
        (return _output_4)
        (else
          (LocalVariables|SetHasVisited_4 true)
          (if (Math|Boolean|ANDBoolean (LocalVariables|GetHasVisited_4) (LocalVariables|GetHasVisited_1) (LocalVariables|GetHasVisited_2) (LocalVariables|GetHasVisited_3))
            (return 0)
            (else
              (goto _label))))))))

(fn IsVisitable
  (params (Tile%20Collision :type BP%20Floor%20Collision%20Object%20Reference))
  (Utilities|IsValid Tile%20Collision
    (:Is%20Valid
      (switch string (Utilities|String|ToString(Text) (Variables|/Script/Engine.TextRenderComponent|GetText (Variables|/Game/PG/Blueprints/BP_FloorCollision.BP_FloorCollision_C|GetIs%20Visitable Tile%20Collision)))
        (:T
          (return true))
        (:F
          _)))
    (:Is%20Not%20Valid
      _))
  (return false))

(fn PushTCStack
  (params (Tile%20Collison :type BP%20Floor%20Collision%20Object%20Reference%20%28by%20ref%29))
  (Rendering|Components|TextRender|SetText (Variables|/Game/PG/Blueprints/BP_FloorCollision.BP_FloorCollision_C|GetIs%20Visitable Tile%20Collison) (LocalVariables|GetLocal%20Value))
  (Utilities|Array|AddUnique (Variables|Default|GetTC_Stack) Tile%20Collison)
  (Math|Integer|IncrementInt (Variables|Default|GetTC_TopPointer)))

(fn PeekTCStack
  (bind _tc_stack (Variables|Default|GetTC_Stack))
  (if (not (Utilities|Array|IsEmpty _tc_stack))
    (return (Utilities|Array|Get(acopy) _tc_stack (Variables|Default|GetTC_TopPointer)))))

(fn GetTileIndex
  (params (Tile%20Collision :type BP%20Floor%20Collision%20Object%20Reference))
  (if (not (Utilities|Array|IsEmpty (Variables|Default|GetTC_Stack)))
    (return (Math|Conversions|ToInteger(Byte) (Utilities|String|ToString(Text) (Variables|/Script/Engine.TextRenderComponent|GetText (Variables|/Game/PG/Blueprints/BP_FloorCollision.BP_FloorCollision_C|GetIndex%20Number Tile%20Collision)))))))

(fn GetBelowTile
  (params (Tile%20Collision :type BP%20Floor%20Collision%20Object%20Reference))
  (bind _returnvalue (CallFunction|GetTileIndex Tile%20Collision))
  (bind _tile_collision_array (Variables|Default|GetTile%20Collision%20Array))
  (bind _returnvalue_2 (+ _returnvalue 1))
  (bind _output (Utilities|Array|Get(acopy) _tile_collision_array _returnvalue_2))
  (Utilities|IsValid _output
    (:Is%20Valid
      (if (== (Math|Integer|%(Integer) _returnvalue_2 (Variables|Default|GetMXCol)) 0)
        (return 0)
        (else
          (return _output))))))

(fn GetAboveTile
  (params (Tile%20Collision :type BP%20Floor%20Collision%20Object%20Reference))
  (bind _returnvalue (CallFunction|GetTileIndex Tile%20Collision))
  (bind _tile_collision_array (Variables|Default|GetTile%20Collision%20Array))
  (bind _returnvalue_2 (- _returnvalue 1))
  (bind _output (Utilities|Array|Get(acopy) _tile_collision_array _returnvalue_2))
  (Utilities|IsValid _output
    (:Is%20Valid
      (if (== (Math|Integer|%(Integer) _returnvalue_2 (Variables|Default|GetMXRow)) 2)
        (return 0)
        (else
          (return _output))))))

(fn GetRightTile
  (params (Tile%20Collision :type BP%20Floor%20Collision%20Object%20Reference))
  (bind _returnvalue (CallFunction|GetTileIndex Tile%20Collision))
  (bind _mxrow (Variables|Default|GetMXRow))
  (bind _tile_collision_array (Variables|Default|GetTile%20Collision%20Array))
  (bind _returnvalue_2 (+ _returnvalue _mxrow))
  (bind _output (Utilities|Array|Get(acopy) _tile_collision_array _returnvalue_2))
  (Utilities|IsValid _output
    (:Is%20Valid
      (return _output))))

(fn GetLeftTile
  (params (Tile%20Collision :type BP%20Floor%20Collision%20Object%20Reference))
  (bind _returnvalue (CallFunction|GetTileIndex Tile%20Collision))
  (bind _mxrow (Variables|Default|GetMXRow))
  (bind _tile_collision_array (Variables|Default|GetTile%20Collision%20Array))
  (bind _returnvalue_2 (- _returnvalue _mxrow))
  (bind _output (Utilities|Array|Get(acopy) _tile_collision_array _returnvalue_2))
  (Utilities|IsValid _output
    (:Is%20Valid
      (return _output))))

(fn PopTCStack
  (bind _tc_toppointer (Variables|Default|GetTC_TopPointer))
  (Utilities|Array|RemoveIndex (Variables|Default|GetTC_Stack) _tc_toppointer)
  (Math|Integer|DecrementInt _tc_toppointer
    (:%20%20
      (Development|PrintString (Utilities|String|Append "Removed: " (Utilities|String|ToString(Integer) (CallFunction|GetTileIndex (CallFunction|PeekTCStack)))) false true "(R=0.000000,G=0.660000,B=1.000000,A=1.000000)" 9e+02))))

(fn SpawnWalls
  (params (Tile%20Collision :type BP%20Floor%20Collision%20Object%20Reference))
  (bind _returnvalue (CallFunction|GetTileIndex Tile%20Collision))
  (bind _floor (Variables|Default|GetFloor))
  (bind (_outinstancetransform _returnvalue_2) (Components|InstancedStaticMesh|GetInstanceTransform _floor _returnvalue true))
  (LocalVariables|SetDifferenceBtwIndex (- _returnvalue (CallFunction|GetTileIndex (CallFunction|PeekTCStack))))
  (Utilities|FlowControl|Sequence
    (:then_0
      (if (== (LocalVariables|GetDifferenceBtwIndex) (Variables|Default|GetMXRow))
        (LocalVariables|SetWallType "NewEnumerator3")
        (switch Utilities|FlowControl|Switch|SwitchonE_WallType (LocalVariables|GetWallType) :!label _label
          (:NewEnumerator0
            (LocalVariables|SetTileOffset "100.000000,100.000000, 0")
            (LocalVariables|SetYaw 0.0))
          (:NewEnumerator1
            (LocalVariables|SetTileOffset "100.000000,-100.000000, 0")
            (LocalVariables|SetYaw 0.0))
          (:NewEnumerator2
            (LocalVariables|SetTileOffset "300.000000,100.000000, 0")
            (LocalVariables|SetYaw 9e+01))
          (:NewEnumerator3
            (LocalVariables|SetTileOffset "100.000000,100.000000, 0")
            (LocalVariables|SetYaw 9e+01)))
        (bind _returnvalue_3 (Components|InstancedStaticMesh|AddInstance (Variables|Default|GetInnerWalls) (Math|Transform|MakeTransform (+ (.location _outinstancetransform) (LocalVariables|GetTileOffset)) (Math|Rotator|MakeRotator (.roll (.rotation _outinstancetransform)) (.pitch (.rotation _outinstancetransform)) (LocalVariables|GetYaw)) (Math|Vector|MakeVector (/ (.x (.scale _outinstancetransform)) 8.0) (.y (.scale _outinstancetransform)) 1.5)) _returnvalue_2))
        (CallFunction|DestroyInnerWalls _returnvalue_3)))
    (:then_1
      (if (== (LocalVariables|GetDifferenceBtwIndex) (* (Variables|Default|GetMXRow) -1))
        (LocalVariables|SetWallType "NewEnumerator2")
        (goto _label)))
    (:then_2
      (if (== (LocalVariables|GetDifferenceBtwIndex) 1)
        (LocalVariables|SetWallType "NewEnumerator1")
        (goto _label)))
    (:then_3
      (if (== (LocalVariables|GetDifferenceBtwIndex) -1)
        (LocalVariables|SetWallType "NewEnumerator0")
        (goto _label)))))

(fn DestroyInnerWalls
  (params (InstanceIndex :type Integer))
  (bind _innerwalls (Variables|Default|GetInnerWalls))
  (for _array_element (Class|PrimitiveComponent|GetOverlappingComponents (Variables|Default|GetWall))
    (bind _asinstanced_static_mesh_component (Utilities|Casting|CastToInstancedStaticMeshComponent _array_element))
    (if (== _asinstanced_static_mesh_component _innerwalls)
      (Class|InstancedStaticMeshComponent|RemoveInstance _innerwalls InstanceIndex))))

(fn SetAllSpwanableTiles
  (for _array_element (Variables|Default|GetTile%20Collision%20Array)
    (bind _can_spawn (Default|GetCanSpawn _array_element))
    (if _can_spawn
      (Utilities|Array|AddUnique (Variables|Default|GetSpawnable%20Tiles) _array_element))))

(fn SpawnCoins
  (bind _spawnable_tiles (Variables|Default|GetSpawnable%20Tiles))
  (bind _returnvalue (Utilities|Array|Length _spawnable_tiles))
  (bind _asbp_maze_game_instance (Utilities|Casting|CastToBP_MazeGameInstance (Game|GetGameInstance)))
  (Variables|/Game/Blueprints/GameInstance/BP_MazeGameInstance.BP_MazeGameInstance_C|SetTotal%20Level%20Keys _asbp_maze_game_instance _returnvalue)
  (bind _index (Utilities|FlowControl|ForLoopwithBreak 0 (- _returnvalue 1))
    (:LoopBody
      (Class|NiagaraComponent|SetAsset (Variables|/Game/PG/Blueprints/BP_FloorCollision.BP_FloorCollision_C|GetCoin (Utilities|Array|Get(acopy) _spawnable_tiles _index)) "/Game/sA_PickupSet_1/Fx/NiagaraSystems/NS_Pickup_1.NS_Pickup_1" true))))