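; BP_FloorCollision is a floor piece for the maze ball game that carries a collectible coin and a spawn-point check.
; When BP_Ball overlaps CoinCollision while the Coin effect uses NS_Pickup_1, it destroys the coin, increments the game instance's acquired keys and calls its level regeneration check.
; GetCanSpawn sphere-tests SpawnablePoint and returns false if any BP_RoomGenerator overlaps it.
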(event OnComponentBeginOverlap(CoinCollision)
  (params (OverlappedComponent :type Primitive%20Component%20Object%20Reference) (OtherActor :type Actor%20Object%20Reference) (OtherComp :type Primitive%20Component%20Object%20Reference) (OtherBodyIndex :type Integer) (bFromSweep :type Boolean) (SweepResult :type Hit%20Result%20Structure%20%28by%20ref%29))
  (bind _coin (Variables|Default|GetCoin))
  ;[1 0.8446 0] Coin Destruction
  (Utilities|Casting|CastToBP_Ball OtherActor)
  (Utilities|IsValid (Variables|Default|GetCoin)
    (:Is%20Valid
      (if (== (AssetData|GetAsset _coin) "/Game/sA_PickupSet_1/Fx/NiagaraSystems/NS_Pickup_1.NS_Pickup_1")
        (Components|DestroyComponent _coin)
        (bind _asbp_maze_game_instance (Utilities|Casting|CastToBP_MazeGameInstance (Game|GetGameInstance)))
        (Math|Integer|IncrementInt (Variables|/Game/Blueprints/GameInstance/BP_MazeGameInstance.BP_MazeGameInstance_C|GetAccquired%20Keys _asbp_maze_game_instance)
          (:%20%20
            (Default|CheckforRegenerateLvl _asbp_maze_game_instance)))))))

(event Collision|EventActorBeginOverlap
  (params (OtherActor :type Actor%20Object%20Reference)))

(fn ConstructionScript)

(fn GetCanSpawn
  (bind _outactors (Collision|SphereOverlapActors (Transformation|GetWorldLocation (Variables|Default|GetSpawnable%20Point)) 3e+01 (Variables|Default|GetObject%20Types) "/Game/PG/Blueprints/BP_RoomGenerator.BP_RoomGenerator_C"))
  (if (> (Utilities|Array|Length _outactors) 0)
    (return false)
    (else
      (return true))))