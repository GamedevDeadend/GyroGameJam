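; BP_RotatingObstacle is an obstacle whose cube the player rotates through input.
; Mobile Tilt (its Y value) and the Move Right axis each add world pitch to the Cube, scaled by RotationRate.
; Both inputs act only while IsRotating is true, and each prints its axis value as a debug string.
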(event EventBeginPlay)

(event Collision|EventActorBeginOverlap
  (params (OtherActor :type Actor%20Object%20Reference)))

(event EventTick
  (params (DeltaSeconds :type Float%20%28single-precision%29)))

(event Input|AxisEvents|InputAxisMoveRight
  (params (AxisValue :type Float%20%28single-precision%29))
  ;[1 1 1] Mobile Obstacle Controls
  (if (Variables|Default|GetIsRotating)
    (Development|PrintString (Utilities|String|Append "Tilt Obstacle Y: " (Utilities|String|ToString(Float) AxisValue)) true true "(R=1.000000,G=0.951325,B=0.000000,A=1.000000)" 0.0)
    (Transformation|AddWorldRotation (Variables|Default|GetCube) (Math|Rotator|MakeRotator 0.0 (* AxisValue (Variables|Default|GetRotation%20Rate)) 0.0) false false)))

(event Input|KeyboardEvents|Tilt
  (params (AxisValue :type Vector :default "0, 0, 0"))
  ;[1 1 1] Mobile Obstacle Controls
  (if (Variables|Default|GetIsRotating)
    (Development|PrintString (Utilities|String|Append "Tilt Obstacle Y: " (Utilities|String|ToString(Float) (.y AxisValue))) true true "(R=1.000000,G=0.951325,B=0.000000,A=1.000000)" 0.0)
    (Transformation|AddWorldRotation (Variables|Default|GetCube) (Math|Rotator|MakeRotator 0.0 (* (.y AxisValue) (Variables|Default|GetRotation%20Rate)) 0.0) false false)))

(fn ConstructionScript)