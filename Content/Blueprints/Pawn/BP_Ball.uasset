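; Ball pawn for a maze game, moved by physics impulses from mobile motion-sensor input.
; Tilt Y continuously pushes the ball mesh along X, scaled by a force multiplier and delta time.
; BP_MazeGameInstance's MotionState selects whether tilt, rotation rate, acceleration or gravity drives the vertical jump.
; The selected sensor's X value, when within the game instance's range, applies its vertical force, with on-screen debug prints throughout.
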(event EventBeginPlay)

(event Collision|EventActorBeginOverlap
  (params (OtherActor :type Actor%20Object%20Reference)))

(event EventTick
  (params (DeltaSeconds :type Float%20%28single-precision%29))
  (Development|PrintString (Utilities|String|Append "Z: " (Utilities|String|ToString(Float) 0.0)) true true "(R=0.000000,G=0.660000,B=1.000000,A=1.000000)" 0.0))

(event Input|KeyboardEvents|Gravity
  (params (AxisValue :type Vector :default "0, 0, 0")))

(event Input|KeyboardEvents|Acceleration
  (params (AxisValue :type Vector :default "0, 0, 0"))
  ;[0 0.3065 1] Gyro Vertical Jump
  (bind _asbp_maze_game_instance (Utilities|Casting|CastToBP_MazeGameInstance (Game|GetGameInstance)))
  (if (Utilities|Enum|Equal(Enum) (Variables|/Game/Blueprints/GameInstance/BP_MazeGameInstance.BP_MazeGameInstance_C|GetMotionState _asbp_maze_game_instance) "NewEnumerator2")
    (Development|PrintString (Utilities|String|Append "Acceleration X: " (Utilities|String|ToString(Float) (.x AxisValue))) true true "(R=0.000000,G=0.660000,B=1.000000,A=1.000000)" 0.0)
    (if (Math|Float|InRange(Float) (.x AxisValue) (Variables|/Game/Blueprints/GameInstance/BP_MazeGameInstance.BP_MazeGameInstance_C|GetMin%20Range _asbp_maze_game_instance) (Variables|/Game/Blueprints/GameInstance/BP_MazeGameInstance.BP_MazeGameInstance_C|GetMax%20Range _asbp_maze_game_instance))
      (Physics|AddImpulse (Variables|Default|GetBallMesh) (Math|Vector|MakeVector 0.0 0.0 (* (Variables|/Game/Blueprints/GameInstance/BP_MazeGameInstance.BP_MazeGameInstance_C|GetVertical%20Force _asbp_maze_game_instance) (Utilities|Time|GetWorldDeltaSeconds))) "None" false))))

(event Input|KeyboardEvents|Gravity
  (params (AxisValue :type Vector :default "0, 0, 0"))
  ;[0 0.3065 1] Gyro Vertical Jump
  (bind _asbp_maze_game_instance (Utilities|Casting|CastToBP_MazeGameInstance (Game|GetGameInstance)))
  (if (Utilities|Enum|Equal(Enum) (Variables|/Game/Blueprints/GameInstance/BP_MazeGameInstance.BP_MazeGameInstance_C|GetMotionState _asbp_maze_game_instance) "NewEnumerator3")
    (Development|PrintString (Utilities|String|Append "Gravity X: " (Utilities|String|ToString(Float) (.x AxisValue))) true true "(R=0.000000,G=0.660000,B=1.000000,A=1.000000)" 0.0)
    (if (Math|Float|InRange(Float) (.x AxisValue) (Variables|/Game/Blueprints/GameInstance/BP_MazeGameInstance.BP_MazeGameInstance_C|GetMin%20Range _asbp_maze_game_instance) (Variables|/Game/Blueprints/GameInstance/BP_MazeGameInstance.BP_MazeGameInstance_C|GetMax%20Range _asbp_maze_game_instance))
      (Physics|AddImpulse (Variables|Default|GetBallMesh) (Math|Vector|MakeVector 0.0 0.0 (* (Variables|/Game/Blueprints/GameInstance/BP_MazeGameInstance.BP_MazeGameInstance_C|GetVertical%20Force _asbp_maze_game_instance) (Utilities|Time|GetWorldDeltaSeconds))) "None" false))))

(event Input|KeyboardEvents|Acceleration
  (params (AxisValue :type Vector :default "0, 0, 0")))

(event Input|KeyboardEvents|RotationRate
  (params (AxisValue :type Vector :default "0, 0, 0")))

(event Input|KeyboardEvents|Tilt
  (params (AxisValue :type Vector :default "0, 0, 0"))
  ;[0.2626 1 0.2764] Horizontal  Gyro Movement
  (Development|PrintString (Utilities|String|Append "Tilt Y: " (Utilities|String|ToString(Float) (.y AxisValue))) true true "(R=0.000000,G=0.660000,B=1.000000,A=1.000000)" 0.0)
  (Physics|AddImpulse (Variables|Default|GetBallMesh) (Math|Vector|MakeVector (* (.y AxisValue) (Variables|Default|GetHorizontal%20Force%20Multiplier) (Utilities|Time|GetWorldDeltaSeconds)) 0.0 0.0) "None" false))

(event Input|KeyboardEvents|Tilt
  (params (AxisValue :type Vector :default "0, 0, 0")))

(event Input|KeyboardEvents|Tilt
  (params (AxisValue :type Vector :default "0, 0, 0"))
  ;[0 0.3065 1] Gyro Vertical Jump
  (bind _asbp_maze_game_instance (Utilities|Casting|CastToBP_MazeGameInstance (Game|GetGameInstance)))
  (if (Utilities|Enum|Equal(Enum) (Variables|/Game/Blueprints/GameInstance/BP_MazeGameInstance.BP_MazeGameInstance_C|GetMotionState _asbp_maze_game_instance) "NewEnumerator1")
    (Development|PrintString (Utilities|String|Append "Tilt X: " (Utilities|String|ToString(Float) (.x AxisValue))) true true "(R=0.000000,G=0.660000,B=1.000000,A=1.000000)" 0.0)
    (if (Math|Float|InRange(Float) (.x AxisValue) (Variables|/Game/Blueprints/GameInstance/BP_MazeGameInstance.BP_MazeGameInstance_C|GetMin%20Range _asbp_maze_game_instance) (Variables|/Game/Blueprints/GameInstance/BP_MazeGameInstance.BP_MazeGameInstance_C|GetMax%20Range _asbp_maze_game_instance))
      (Physics|AddImpulse (Variables|Default|GetBallMesh) (Math|Vector|MakeVector 0.0 0.0 (* (Variables|/Game/Blueprints/GameInstance/BP_MazeGameInstance.BP_MazeGameInstance_C|GetVertical%20Force _asbp_maze_game_instance) (Utilities|Time|GetWorldDeltaSeconds))) "None" false))))

(event Input|KeyboardEvents|RotationRate
  (params (AxisValue :type Vector :default "0, 0, 0"))
  ;[0 0.3065 1] Gyro Vertical Jump
  (bind _asbp_maze_game_instance (Utilities|Casting|CastToBP_MazeGameInstance (Game|GetGameInstance)))
  (if (Utilities|Enum|Equal(Enum) (Variables|/Game/Blueprints/GameInstance/BP_MazeGameInstance.BP_MazeGameInstance_C|GetMotionState _asbp_maze_game_instance) "NewEnumerator0")
    (Development|PrintString (Utilities|String|Append "Rotation X: " (Utilities|String|ToString(Float) (.x AxisValue))) true true "(R=0.000000,G=0.660000,B=1.000000,A=1.000000)" 0.0)
    (if (Math|Float|InRange(Float) (.x AxisValue) (Variables|/Game/Blueprints/GameInstance/BP_MazeGameInstance.BP_MazeGameInstance_C|GetMin%20Range _asbp_maze_game_instance) (Variables|/Game/Blueprints/GameInstance/BP_MazeGameInstance.BP_MazeGameInstance_C|GetMax%20Range _asbp_maze_game_instance))
      (Physics|AddImpulse (Variables|Default|GetBallMesh) (Math|Vector|MakeVector 0.0 0.0 (* (Variables|/Game/Blueprints/GameInstance/BP_MazeGameInstance.BP_MazeGameInstance_C|GetVertical%20Force _asbp_maze_game_instance) (Utilities|Time|GetWorldDeltaSeconds))) "None" false))))

(fn ConstructionScript)