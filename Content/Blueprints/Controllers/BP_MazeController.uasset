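; BP_MazeController is a controller that switches control between the ball and the maze.
; It possesses the BP_Ball found in the level on BeginPlay.
; The SwitchControls event uses a FlipFlop to unpossess the current pawn and possess the first BP_Maze or BP_Ball found, alternating on each call, starting with the maze.
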(event Custom|Switch%20Controls
  (Utilities|FlowControl|FlipFlop
    (:A
      (Pawn|UnPossess)
      (bind _outactors (Actor|GetAllActorsOfClass "/Game/Blueprints/Maze/BP_Maze.BP_Maze_C"))
      (Pawn|Possess (Utilities|Array|Get(acopy) _outactors)))
    (:B
      (Pawn|UnPossess)
      (bind _outactors_2 (Actor|GetAllActorsOfClass "/Game/Blueprints/Pawn/BP_Ball.BP_Ball_C"))
      (Pawn|Possess (Utilities|Array|Get(acopy) _outactors_2)))))

(event EventBeginPlay
  (bind _returnvalue (Actor|GetActorOfClass "/Game/Blueprints/Pawn/BP_Ball.BP_Ball_C"))
  (Pawn|Possess _returnvalue))

(event EventTick
  (params (DeltaSeconds :type Float%20%28single-precision%29)))

(fn ConstructionScript)